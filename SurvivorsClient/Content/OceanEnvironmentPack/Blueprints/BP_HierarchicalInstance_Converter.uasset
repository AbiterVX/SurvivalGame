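; Runtime converter actor that replaces all actors carrying a given tag with instances in a single HierarchicalInstancedStaticMesh.
; On BeginPlay it moves to the world origin so gathered world transforms can serve as instance transforms, assigns the configured mesh, then adds an instance per tagged actor.
; It then destroys the original actors.
; The construction script applies the configured material to the first slot.
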(event EventBeginPlay
  (Transformation|SetActorLocation "0, 0, 0" false false)
  (Components|StaticMesh|SetStaticMesh (Variables|Default|GetHierarchicalInstancedStaticMesh) (Variables|Default|GetStaticMesh))
  (bind _outactors (Actor|GetAllActorswithTag (Utilities|String|StringToName (Variables|Default|GetTag))))
  (for _array_element _outactors
    (Utilities|Array|Add (Variables|Default|GetArray) _array_element)
    (Utilities|Array|Add (Variables|Default|GetTransform) (Transformation|GetActorTransform _array_element)))
  (for _array_element_2 (Variables|Default|GetTransform)
    (Components|InstancedStaticMesh|AddInstance (Variables|Default|GetHierarchicalInstancedStaticMesh) _array_element_2))
  (for _array_element_3 (Variables|Default|GetArray)
    (if (Utilities|IsValid _array_element_3)
      (Actor|DestroyActor _array_element_3))))

(event Collision|EventActorBeginOverlap
  (params (OtherActor :type Actor%20Object%20Reference)))

(event EventTick
  (params (DeltaSeconds :type Float%20%28single-precision%29)))

(fn ConstructionScript
  (Rendering|Material|SetMaterial (Variables|Default|GetHierarchicalInstancedStaticMesh) 0 (Variables|Default|GetMaterial_Element0)))