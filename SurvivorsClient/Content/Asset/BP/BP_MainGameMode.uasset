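; Main game mode that caches world actors and manages the game's UI widgets.
; On BeginPlay it stores the game instance, world timer, sun, sky sphere and skylight, then shows the main, aim and inventory widgets.
; Helper functions show, hide and look up widgets in a keyed map, and return the timer's time as text.
; Sun rotation, sky update, quit and restart logic is present but unconnected.
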(event EventBeginPlay
  (if true
    (Utilities|FlowControl|Sequence
      (:then_0
        ;[1 1 1] 设置GameInstance
        (Variables|Default|SetBP_MainGameInstance (.AsBP%20Main%20Game%20Instance (Utilities|Casting|CastToBP_MainGameInstance (Game|GetGameInstance)))))
      (:then_1
        ;[1 1 1] WorldTimer
        (bind _returnvalue (Actor|GetActorOfClass "/Script/Nature.WorldTimer"))
        (Variables|Default|SetCurrentWorldTimer _returnvalue))
      (:then_2
        ;[1 1 1] DirectionalLight
        (bind _returnvalue_2 (Actor|GetActorOfClass "/Script/Engine.DirectionalLight"))
        (Variables|Default|SetSun _returnvalue_2))
      (:then_3
        ;[1 1 1] SkySphere
        (bind _returnvalue_3 (Actor|GetActorOfClass "/Engine/EngineSky/BP_Sky_Sphere.BP_Sky_Sphere_C"))
        (Variables|Default|SetSkySphere _returnvalue_3))
      (:then_4
        ;[1 1 1] SkyLight
        (bind _returnvalue_4 (Actor|GetActorOfClass "/Script/Engine.SkyLight"))
        (Variables|Default|SetSkyLight _returnvalue_4))
      (:then_5
        ;[1 1 1] 显示UI
        (Utilities|FlowControl|Sequence
          (:then_0
            ;;[1 1 1] 显示UIMain界面
            (CallFunction|FunShowUIWidget "/Game/Asset/BP/UI/UIMain.UIMain_C" "UIMain"))
          (:then_1
            ;;[1 1 1] 显示UIAim界面
            (CallFunction|FunShowUIWidget "/Game/Asset/BP/UI/UIAim.UIAim_C" "UIAim"))
          (:then_2
            ;;[1 1 1] 显示UIInventory界面
            (CallFunction|FunShowUIWidget "/Game/Asset/BP/UI/UIInventory.UIInventory_C" "UIInventory")))))))

(event EventTick
  (params (DeltaSeconds :type Float%20%28single-precision%29)))

(fn ConstructionScript)

(fn FunShowUIWidget
  (params (UserWidgetClass :type User%20Widget%20Class%20Reference) (Key :type String))
  (bind _returnvalue (UserInterface|CreateWidget UserWidgetClass (Game|GetPlayerController 0)))
  (UserInterface|Viewport|AddtoViewport _returnvalue 0)
  (Utilities|Map|Add (Variables|Default|GetUIWidgetInsts) Key _returnvalue))

(fn FunHideUIWidget
  (params (Key :type String))
  (bind _uiwidgetinsts (Variables|Default|GetUIWidgetInsts))
  (bind (_value _returnvalue) (Utilities|Map|Find _uiwidgetinsts Key))
  (if _returnvalue
    (Widget|RemovefromParent _value)))

(fn FunGetUIWidgetInst
  (params (Key :type String))
  (return (.Value (Utilities|Map|Find (Variables|Default|GetUIWidgetInsts) Key))))

(fn FunGetCurrentTime
  (bind _currentworldtimer (Variables|Default|GetCurrentWorldTimer))
  (if (Utilities|IsValid _currentworldtimer)
    (bind _returnvalue (Class|WorldTimer|GetGameTimeinFString _currentworldtimer))
    (return _returnvalue)
    (else
      (return "None"))))

(fn FunGetTimeState
  (bind _returnvalue (Class|WorldTimer|GetCurrentDayPercent (Variables|Default|GetCurrentWorldTimer))))