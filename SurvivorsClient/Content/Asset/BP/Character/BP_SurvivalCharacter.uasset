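; Player survival character Blueprint handling item interaction, inventory, running camera shake, swim rotation, ragdoll death and base building.
; Capsule overlaps track nearby items, driving aim-UI tips and nearest-item interaction, while inventory input refreshes or toggles widgets fetched from the GameMode.
; In build mode, a per-tick camera trace snaps the preview to matching slot actors and swaps its validity material.
; Clicking consumes the slots and spawns another preview; only floors are implemented.
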(event OnComponentBeginOverlap(CapsuleCollison)
  (params (OverlappedComponent :type Primitive%20Component%20Object%20Reference) (OtherActor :type Actor%20Object%20Reference) (OtherComp :type Primitive%20Component%20Object%20Reference) (OtherBodyIndex :type Integer) (bFromSweep :type Boolean) (SweepResult :type Hit%20Result%20Structure%20%28by%20ref%29))
  ;[1 1 1] Collision:BeginOverlap
  (bind _asitem (Utilities|Casting|CastToItem OtherActor))
  (Utilities|FlowControl|Sequence
    (:then_0
      ;;[1 1 1] 添加OverLap的Item
      (Class|SurvivalCharacter|AddOverlapItem _asitem))
    (:then_1
      ;;[1 1 1] 转为UIAim
      (bind _asbp_main_game_mode (Utilities|Casting|CastToBP_MainGameMode (Game|GetGameMode)))
      (if (.ReturnValue (Utilities|Map|Find (Variables|/Game/Asset/BP/BP_MainGameMode.BP_MainGameMode_C|GetUIWidgetInsts _asbp_main_game_mode) "UIAim"))
        (bind _asuiaim (Utilities|Casting|CastToUIAim (.Value (Utilities|Map|Find (Variables|/Game/Asset/BP/BP_MainGameMode.BP_MainGameMode_C|GetUIWidgetInsts _asbp_main_game_mode) "UIAim"))))
        ;;[1 1 1] 显示距离最近Item的Tips
        (bind _returnvalue (Class|SurvivalCharacter|GetNearestOverlapItem))
        (Default|FunShowTips _asuiaim "Visible" _returnvalue)))))

(event OnComponentEndOverlap(CapsuleCollison)
  (params (OverlappedComponent :type Primitive%20Component%20Object%20Reference) (OtherActor :type Actor%20Object%20Reference) (OtherComp :type Primitive%20Component%20Object%20Reference) (OtherBodyIndex :type Integer))
  ;[1 1 1] Collision:End OverLap
  ;;[1 1 1] 移除不再Overlap的Item
  (bind _asitem (Utilities|Casting|CastToItem OtherActor))
  (Class|SurvivalCharacter|RemoveOverlapItem _asitem)
  ;;[1 1 1] 转为UIAim
  (bind _asbp_main_game_mode (Utilities|Casting|CastToBP_MainGameMode (Game|GetGameMode)))
  (if (.ReturnValue (Utilities|Map|Find (Variables|/Game/Asset/BP/BP_MainGameMode.BP_MainGameMode_C|GetUIWidgetInsts _asbp_main_game_mode) "UIAim"))
    (bind _asuiaim (Utilities|Casting|CastToUIAim (.Value (Utilities|Map|Find (Variables|/Game/Asset/BP/BP_MainGameMode.BP_MainGameMode_C|GetUIWidgetInsts _asbp_main_game_mode) "UIAim"))))
    ;;[1 1 1] 显示/隐藏Tips
    (bind _returnvalue (Class|SurvivalCharacter|GetNearestOverlapItem))
    (if (Utilities|IsValid _returnvalue)
      (Default|FunShowTips _asuiaim "Visible" _returnvalue)
      (else
        (Default|FunHideTips _asuiaim)))))

(event Custom|Event_CharacterDead
  ;[1 1 1] Event:死亡
  (Input|DisableInput (Game|GetPlayerController 0))
  (Variables|/Script/Engine.PlayerController|SetbShowMouseCursor (Game|GetPlayerController 0) true)
  ;;[1 1 1] 物理模拟与权重设置
  (Class|SkeletalMeshComponent|SetAllBodiesSimulatePhysics (Variables|Character|GetMesh) true)
  (Class|SkeletalMeshComponent|SetAllBodiesPhysicsBlendWeight (Variables|Character|GetMesh) 1.0 false)
  ;;[1 1 1] 设置碰撞
  (Collision|SetCollisionEnabled (Variables|Character|GetMesh) "QueryAndPhysics"))

(event Custom|Event_BuildTrace
  (bind _returnvalue (Game|GetPlayerCameraManager 0))
  (bind _currentbuilditem (Variables|Build|GetCurrentBuildItem))
  (bind _currentbuilditem_2 (Variables|Build|GetCurrentBuildItem))
  (bind _returnvalue_2 (Transformation|GetActorForwardVector _returnvalue))
  (bind _returnvalue_3 (Math|Conversions|RotationFromXVector (Math|Vector|MakeVector (.x _returnvalue_2) (.y _returnvalue_2) 0.0)))
  ;[1 1 1] Event:建造射线检测
  (if (Variables|Build|GetBuildMode)
    (bind (_startlocation _endlocation) (CallFunction|FunGetBuildTraceLocation))
    (bind (_outhit _returnvalue_4) (Collision|LineTraceByChannel _startlocation _endlocation "TraceTypeQuery3" false (Utilities|Array|MakeArray (Variables|Build|GetCurrentBuildItem)) "ForOneFrame"))
    (if _returnvalue_4
      (bind _asbp_build_item_slot (Utilities|Casting|CastToBP_BuildItemSlot (.HitActor (Collision|BreakHitResult _outhit)))
        (:then
          (bind _name (CallFunction|FunGetSlotType (Variables|Build|GetCurrentBuildItemType)))
          (if (and (Utilities|Enum|Equal(Enum) _name (Variables|/Game/Asset/BP/Item/BP_BuildItemSlot.BP_BuildItemSlot_C|GetSlotType _asbp_build_item_slot)) (!= (Actor|GetParentActor _asbp_build_item_slot) (Variables|Build|GetCurrentBuildItem)))
            (Variables|Build|SetCurrentBuildItemSlot _asbp_build_item_slot)
            (bind _asbp_build_item (Utilities|Casting|CastToBP_BuildItem (Actor|GetParentActor _asbp_build_item_slot)))
            (Transformation|SetActorTransform _currentbuilditem (Math|Transform|MakeTransform (|(Location+(Direction*EdgeLength)) (Transformation|GetActorLocation _asbp_build_item) (* (Transformation|GetActorForwardVector _asbp_build_item_slot) -1.0) (Variables|/Game/Asset/BP/Item/BP_BuildItem.BP_BuildItem_C|GetEdgeLength _asbp_build_item)) (Transformation|GetActorRotation _asbp_build_item)))
            (Default|FunSetMainBuildItemMaterial _currentbuilditem "CanPlace")))
        (:CastFailed
          (Transformation|SetActorTransform _currentbuilditem_2 (Math|Transform|MakeTransform (.Location (Collision|BreakHitResult _outhit)) _returnvalue_3))
          (Default|FunSetMainBuildItemMaterial _currentbuilditem_2 "CanNotPlace")))
      (else
        (Transformation|SetActorTransform _currentbuilditem_2 (Math|Transform|MakeTransform _endlocation _returnvalue_3))
        (Default|FunSetMainBuildItemMaterial _currentbuilditem_2 "CanNotPlace")))))

(event Custom|Event_CameraShake
  (bind _charactermovement (Variables|Character|GetCharacterMovement))
  ;[1 1 1] Event:相机晃动
  (if (and (Utilities|Enum|Equal(Enum) (Variables|/Script/Engine.CharacterMovementComponent|GetMovementMode _charactermovement) "MOVE_Walking") (> (Math|Vector|VectorLength (Variables|/Script/Engine.MovementComponent|GetVelocity _charactermovement)) 4e+02))
    (Class|PlayerCameraManager|PlayCameraShake (Game|GetPlayerCameraManager 0) "/Game/Asset/BP/Character/BP_CameraShake_Run.BP_CameraShake_Run_C" 5.0 "CameraLocal" "0, 0, 0")))

(event Custom|Event_BuidOneItem
  (bind _returnvalue (Game|GetPlayerCameraManager 0))
  (bind _returnvalue_2 (Transformation|GetActorForwardVector _returnvalue))
  ;[1 1 1] Event:建造一个BuildItem
  ;;[1 1 1] MakeTransform
  (bind _endlocation (CallFunction|FunGetBuildTraceLocation))
  (switch string (Variables|Build|GetCurrentBuildItemType)
    (:Floor
      (bind _returnvalue_3 (Game|SpawnActorfromClass "/Game/Asset/BP/Item/BP_BuildItem_Floor.BP_BuildItem_Floor_C" (Math|Transform|MakeTransform _endlocation (Math|Conversions|RotationFromXVector (Math|Vector|MakeVector (.x _returnvalue_2) (.y _returnvalue_2) 0.0))) "Undefined" 0 0))
      (Variables|Build|SetCurrentBuildItem _returnvalue_3))))

(event EventBeginPlay)

(event Collision|EventActorBeginOverlap
  (params (OtherActor :type Actor%20Object%20Reference)))

(event EventTick
  (params (DeltaSeconds :type Float%20%28single-precision%29))
  ;[1 1 1] Event:Tick
  (|CallParentFunction DeltaSeconds)
  ;;[1 1 1] 相机晃动
  (CallFunction|EventCameraShake)
  ;;[1 1 1] 建造射线检测
  (CallFunction|EventBuildTrace))

(event EventOnMovementModeChanged
  (params (PrevMovementMode :type EMovementMode%20Enum :default "MOVE_None") (NewMovementMode :type EMovementMode%20Enum :default "MOVE_None") (PrevCustomMode :type Byte :default 0) (NewCustomMode :type Byte :default 0))
  (bind _charactermovement (Variables|Character|GetCharacterMovement))
  ;[1 1 1] Event MovementModeChanged:运动Mode改变,Swim
  (if (Utilities|Enum|Equal(Enum) NewMovementMode "MOVE_Swimming")
    (Variables|/Script/Engine.CharacterMovementComponent|SetRotationRate _charactermovement "360.000000,360.000000,360.000000")
    (Variables|Default|SetbUseControllerRotationYaw false)
    (else
      (Variables|/Script/Engine.CharacterMovementComponent|SetRotationRate _charactermovement "0,360.000000, 0")
      (Variables|Default|SetbUseControllerRotationYaw true)
      (Transformation|SetActorRotation (Math|Rotator|MakeRotator 0.0 0.0 (.yaw (Transformation|GetActorRotation)))))))

(event Input|ActionEvents|InputActionInteract
  (params (Key :type Key%20Structure :default "None"))
  ;[1 1 1] Input:按E 交互
  (:Pressed
    ;;[1 1 1] 与距离最近的Item交互
    (bind _returnvalue (Class|SurvivalCharacter|GetNearestOverlapItem))
    (Class|SurvivalCharacter|InteractCurrentItem _returnvalue 1)
    ;;[1 1 1] 获取UIInventory
    (bind _asbp_main_game_mode (Utilities|Casting|CastToBP_MainGameMode (Game|GetGameMode)))
    (bind _value (Default|FunGetUIWidgetInst _asbp_main_game_mode "UIInventory"))
    (bind _asuiinventory (Utilities|Casting|CastToUIInventory _value))
    (Default|EventRefreshAllInventory _asuiinventory)))

(event Input|ActionEvents|InputActionInventoryMain
  (params (Key :type Key%20Structure :default "None"))
  ;[1 1 1] Input:按Tab
  (:Pressed
    ;;[1 1 1] InventoryMainState
    (bind _output_get (Variables|Default|SetinventoryMainState (not (Variables|Default|GetinventoryMainState))))
    ;;[1 1 1] 显示/隐藏鼠标
    (Variables|/Script/Engine.PlayerController|SetbShowMouseCursor (Game|GetPlayerController 0) (not _output_get))
    ;;[1 1 1] 获取UIInventoryInst
    (bind _asbp_main_game_mode (Utilities|Casting|CastToBP_MainGameMode (Game|GetGameMode)))
    (bind _value (Default|FunGetUIWidgetInst _asbp_main_game_mode "UIInventory"))
    (bind _asuiinventory (Utilities|Casting|CastToUIInventory _value))
    ;;[1 1 1] 显示/隐藏背包详情
    (if (not _output_get)
      (Default|EventShowInventoryDetail _asuiinventory)
      (else
        (Default|EventHideInventoryDetail _asuiinventory)))))

(event Input|ActionEvents|InputActionDiscard
  (params (Key :type Key%20Structure :default "None"))
  ;[1 1 1] Input:按Q,丢弃
  (:Pressed
    (Utilities|FlowControl|Sequence
      (:then_0
        ;;[1 1 1] 打印消息
        (bind _asbp_main_game_mode (Utilities|Casting|CastToBP_MainGameMode (Game|GetGameMode)))
        (bind _value (Default|FunGetUIWidgetInst _asbp_main_game_mode "UIMain"))
        (bind _asuimain (Utilities|Casting|CastToUIMain _value))
        (Default|EventAddMessage _asuimain (Utilities|Text|ToText(String) (Utilities|String|Append "移除物品，ID:" (Utilities|String|ToString(Integer) (Variables|/Script/WorldItem.Item|GetitemId (Variables|Default|GetcurrentItemInRightHands)))))))
      (:then_1
        (Class|SurvivalCharacter|DiscardCurrentItem)
        ;;[1 1 1] 获取UIInventory
        (bind _asbp_main_game_mode_2 (Utilities|Casting|CastToBP_MainGameMode (Game|GetGameMode)))
        (bind _value_2 (Default|FunGetUIWidgetInst _asbp_main_game_mode_2 "UIInventory"))
        (bind _asuiinventory (Utilities|Casting|CastToUIInventory _value_2))
        (Default|EventRefreshAllInventory _asuiinventory)))))

(event Input|ActionEvents|InputActionBuild
  (params (Key :type Key%20Structure :default "None"))
  ;[1 1 1] Input:Build
  (:Pressed
    (bind _output_get (Variables|Build|SetBuildMode (not (Variables|Build|GetBuildMode))))
    (if _output_get
      (CallFunction|EventBuidOneItem)
      (else
        (Actor|DestroyActor (Variables|Build|GetCurrentBuildItem))))))

(event Input|ActionEvents|InputActionUseItem_1
  (params (Key :type Key%20Structure :default "None"))
  (bind _currentbuilditemslot (Variables|Build|GetCurrentBuildItemSlot))
  ;[1 1 1] Input: MouseLeftButton
  (:Pressed
    ;;[1 1 1] 放置
    (if (Variables|Build|GetBuildMode)
      (bind _asbp_build_item (Utilities|Casting|CastToBP_BuildItem (Actor|GetParentActor _currentbuilditemslot)))
      (bind _asbp_build_item_floor (Utilities|Casting|CastToBP_BuildItem_Floor (Variables|Build|GetCurrentBuildItem)))
      (Default|FunDeleteSlotbyDirection _asbp_build_item_floor (Math|Vector|Normalize (- (Transformation|GetActorLocation _asbp_build_item) (Transformation|GetActorLocation _currentbuilditemslot))))
      (Actor|DestroyActor _currentbuilditemslot)
      (Default|FunDeleteOverlapSameFloorSlot _asbp_build_item_floor)
      (Default|FunSetMainBuildItemMaterial _asbp_build_item_floor "Origin")
      (CallFunction|EventBuidOneItem))))

(fn ConstructionScript
  (|CallParentFunction)
  (Components|Capsule|SetCapsuleHalfHeight (Variables|Default|GetCapsuleComponent) 88.0 true))

(fn FunGetBuildSlotType
  (params (Type :type String))
  (switch string Type
    (:Floor
      _)
    (:Wall
      _)
    (:Pillar
      (return "TraceTypeQuery5")))
  (return "TraceTypeQuery4"))

(fn FunGetBuildTraceLocation
  (bind _returnvalue (Game|GetPlayerCameraManager 0))
  (bind _buildtracestartlength (Variables|Build|GetBuildTraceStartLength))
  (bind _returnvalue_2 (Transformation|GetActorLocation _returnvalue))
  (bind _returnvalue_3 (Transformation|GetActorForwardVector _returnvalue))
  (bind _returnvalue_4 (|(Location+(Forward*StartLength)) _returnvalue_2 _returnvalue_3 _buildtracestartlength))
  (return _returnvalue_4 (|(StartLocation+(Forward*Length)) _returnvalue_4 _returnvalue_3 (Variables|Build|GetBuildTraceLength))))

(fn FunGetSlotType
  (params (Selection :type String))
  (switch string Selection
    (:Floor
      _)
    (:Wall
      _)
    (:Pillar
      (return "Corner")))
  (return "Edge"))