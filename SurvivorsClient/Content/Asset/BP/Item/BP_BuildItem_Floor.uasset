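; Floor piece for a building system, with a Main component, four edge slots and an edge length set at construction.
; Deleting by direction compares the given vector to Main's forward and right axes, both signs, and destroys the matching edge slot component.
; Overlap cleanup box-queries each edge slot's bounds and destroys intersecting build slot actors that belong to other actors.
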(event EventBeginPlay
  (|CallParentFunction) ; This node is disabled and will not be called.\nDrag off pins to build functionality.
)

(event Collision|EventActorBeginOverlap
  (params (OtherActor :type Actor%20Object%20Reference))
  (|CallParentFunction OtherActor) ; This node is disabled and will not be called.\nDrag off pins to build functionality.
)

(event EventTick
  (params (DeltaSeconds :type Float%20%28single-precision%29))
  (|CallParentFunction DeltaSeconds) ; This node is disabled and will not be called.\nDrag off pins to build functionality.
)

(fn ConstructionScript
  (|CallParentFunction)
  (Variables|Default|SetEdgeLength 2e+02))

(fn FunDeleteSlotbyDirection
  (params (Direction :type Vector))
  (bind _main (Variables|Default|GetMain))
  (Utilities|FlowControl|Sequence
    (:then_0
      (Utilities|MacroDeleteSlotbyDirecion Direction (* (Math|Vector|GetForwardVector _main) -1.0) (Variables|Default|GetSlot_Edge_1)))
    (:then_1
      (Utilities|MacroDeleteSlotbyDirecion Direction (Math|Vector|GetRightVector _main) (Variables|Default|GetSlot_Edge_2)))
    (:then_2
      (Utilities|MacroDeleteSlotbyDirecion Direction (Math|Vector|GetForwardVector _main) (Variables|Default|GetSlot_Edge_3)))
    (:then_3
      (Utilities|MacroDeleteSlotbyDirecion Direction (* (Math|Vector|GetRightVector _main) -1.0) (Variables|Default|GetSlot_Edge_4)))))

(fn FunDeleteOverlapSameFloorSlot
  (Utilities|FlowControl|Sequence
    (:then_0
      (Utilities|MacroDeleteOverlapSameFloorSlot (Variables|Default|GetSlot_Edge_1)))
    (:then_1
      (Utilities|MacroDeleteOverlapSameFloorSlot (Variables|Default|GetSlot_Edge_2)))
    (:then_2
      (Utilities|MacroDeleteOverlapSameFloorSlot (Variables|Default|GetSlot_Edge_3)))
    (:then_3
      (Utilities|MacroDeleteOverlapSameFloorSlot (Variables|Default|GetSlot_Edge_4)))))

(fn FunGetBuildItemMain
  (return (Variables|Default|GetMain)))